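; Gate is a double-door Blueprint in BoulderDash that swings open when its UnlockSelf event fires.
; A timeline yaws the two door meshes up to 90 degrees in opposite directions while a 2D choir sound plays.
; When the timeline finishes, it calls FadeOut on the first actor found implementing the I_FadeOut interface.
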(event EventUnlockSelf
  (Utilities|FlowControl|Sequence
    (:then_0
      (bind _door_opening (Timeline|Open%20Gate%20Timeline Play)
        (:Update
          (Transformation|SetRelativeRotation (Variables|Default|GetCanneryPalaceDoor_a) (Math|Rotator|MakeRotator 0.0 0.0 (* _door_opening -9e+01)) false false)
          (Transformation|SetRelativeRotation (Variables|Default|GetCanneryPalaceDoor_b) (Math|Rotator|MakeRotator 0.0 0.0 (* (* _door_opening -9e+01) -1.0)) false false))
        (:Finished
          (bind _outactors (Actor|GetAllActorswithInterface "/Game/BoulderDash/Interfaces/I_FadeOut.I_FadeOut_C"))
          (bind _asi_fade_out (Utilities|Casting|CastToI_FadeOut (Utilities|Array|Get(acopy) _outactors)))
          (Default|FadeOut _asi_fade_out))))
    (:then_1
      (Audio|PlaySound2D "/Game/BoulderDash/Sounds/angelchoirmarktreekort.angelchoirmarktreekort" 1.0 1.0 0.0 0 0))))

(fn ConstructionScript)