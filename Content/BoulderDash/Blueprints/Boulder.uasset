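; Grid-based Boulder Dash boulder that falls, rolls off supporting actors, kills killable pawns beneath it and can be pushed sideways.
; Five collider boxes detect free neighbouring cells and feed debug text; end-overlap events retrigger TryFallDown.
; If blocked below by an I_CanFallOff actor, it randomly prefers a side, moving sideways then down.
; Timelines animate the Sphere's relative offset, then the actor location jumps one GridSize step.
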(event OnComponentEndOverlap(ColliderBoxDown)
  (params (OverlappedComponent :type Primitive%20Component%20Object%20Reference) (OtherActor :type Actor%20Object%20Reference) (OtherComp :type Primitive%20Component%20Object%20Reference) (OtherBodyIndex :type Integer))
  (if (Variables|Default|GetMoving)
    (CallFunction|UpdateDebugText)
    (else
      (CallFunction|UpdateDebugText)
      (Utilities|FlowControl|RetriggerableDelay 0.5)
      (CallFunction|TryFallDown))))

(event OnComponentBeginOverlap(ColliderBoxDown)
  (params (OverlappedComponent :type Primitive%20Component%20Object%20Reference) (OtherActor :type Actor%20Object%20Reference) (OtherComp :type Primitive%20Component%20Object%20Reference) (OtherBodyIndex :type Integer) (bFromSweep :type Boolean) (SweepResult :type Hit%20Result%20Structure%20%28by%20ref%29))
  (CallFunction|UpdateDebugText))

(event OnComponentEndOverlap(ColliderBoxLeftDown)
  (params (OverlappedComponent :type Primitive%20Component%20Object%20Reference) (OtherActor :type Actor%20Object%20Reference) (OtherComp :type Primitive%20Component%20Object%20Reference) (OtherBodyIndex :type Integer))
  (CallFunction|UpdateDebugText)
  (CallFunction|TryFallDown))

(event OnComponentBeginOverlap(ColliderBoxRightDown)
  (params (OverlappedComponent :type Primitive%20Component%20Object%20Reference) (OtherActor :type Actor%20Object%20Reference) (OtherComp :type Primitive%20Component%20Object%20Reference) (OtherBodyIndex :type Integer) (bFromSweep :type Boolean) (SweepResult :type Hit%20Result%20Structure%20%28by%20ref%29))
  (CallFunction|UpdateDebugText))

(event OnComponentEndOverlap(ColliderBoxRightDown)
  (params (OverlappedComponent :type Primitive%20Component%20Object%20Reference) (OtherActor :type Actor%20Object%20Reference) (OtherComp :type Primitive%20Component%20Object%20Reference) (OtherBodyIndex :type Integer))
  (CallFunction|UpdateDebugText)
  (CallFunction|TryFallDown))

(event OnComponentBeginOverlap(ColliderBoxRight)
  (params (OverlappedComponent :type Primitive%20Component%20Object%20Reference) (OtherActor :type Actor%20Object%20Reference) (OtherComp :type Primitive%20Component%20Object%20Reference) (OtherBodyIndex :type Integer) (bFromSweep :type Boolean) (SweepResult :type Hit%20Result%20Structure%20%28by%20ref%29))
  (CallFunction|UpdateDebugText))

(event OnComponentBeginOverlap(ColliderBoxLeft)
  (params (OverlappedComponent :type Primitive%20Component%20Object%20Reference) (OtherActor :type Actor%20Object%20Reference) (OtherComp :type Primitive%20Component%20Object%20Reference) (OtherBodyIndex :type Integer) (bFromSweep :type Boolean) (SweepResult :type Hit%20Result%20Structure%20%28by%20ref%29))
  (CallFunction|UpdateDebugText))

(event OnComponentBeginOverlap(ColliderBoxLeftDown)
  (params (OverlappedComponent :type Primitive%20Component%20Object%20Reference) (OtherActor :type Actor%20Object%20Reference) (OtherComp :type Primitive%20Component%20Object%20Reference) (OtherBodyIndex :type Integer) (bFromSweep :type Boolean) (SweepResult :type Hit%20Result%20Structure%20%28by%20ref%29))
  (CallFunction|UpdateDebugText))

(event OnComponentEndOverlap(ColliderBoxRight)
  (params (OverlappedComponent :type Primitive%20Component%20Object%20Reference) (OtherActor :type Actor%20Object%20Reference) (OtherComp :type Primitive%20Component%20Object%20Reference) (OtherBodyIndex :type Integer))
  (CallFunction|UpdateDebugText)
  (CallFunction|TryFallDown))

(event OnComponentEndOverlap(ColliderBoxLeft)
  (params (OverlappedComponent :type Primitive%20Component%20Object%20Reference) (OtherActor :type Actor%20Object%20Reference) (OtherComp :type Primitive%20Component%20Object%20Reference) (OtherBodyIndex :type Integer))
  (CallFunction|UpdateDebugText)
  (CallFunction|TryFallDown))

(event Custom|UpdateDebugText
  ;[1 1 1] Debug text
  (Rendering|Components|TextRender|SetText (Variables|Default|GetDebugText) (Utilities|Text|ToText(String) (Utilities|String|JoinStringArray (Utilities|Array|MakeArray (Utilities|String|MakeLiteralString " 
") (Utilities|String|SelectString "O" "X" (== (Utilities|Array|Length (Collision|GetOverlappingActors (Variables|Default|GetColliderBox%20Left) 0 :!class /Script/Engine.PrimitiveComponent)) 0)) (Utilities|String|MakeLiteralString "  ") (Utilities|String|SelectString "O" "X" (== (Utilities|Array|Length (Collision|GetOverlappingActors (Variables|Default|GetColliderBox%20Right) 0 :!class /Script/Engine.PrimitiveComponent)) 0)) (Utilities|String|MakeLiteralString " 
") (Utilities|String|SelectString "O" "X" (== (Utilities|Array|Length (Collision|GetOverlappingActors (Variables|Default|GetColliderBox%20LeftDown) 0 :!class /Script/Engine.PrimitiveComponent)) 0)) (Utilities|String|SelectString "O" "X" (== (Utilities|Array|Length (Collision|GetOverlappingActors (Variables|Default|GetColliderBox%20Down) 0 :!class /Script/Engine.PrimitiveComponent)) 0)) (Utilities|String|SelectString "O" "X" (== (Utilities|Array|Length (Collision|GetOverlappingActors (Variables|Default|GetColliderBox%20RightDown) 0 :!class /Script/Engine.PrimitiveComponent)) 0))) " "))))

(event Custom|Try%20Fall%20Down
  (bind _returnvalue (Transformation|GetActorTransform))
  (bind _returnvalue_2 (Transformation|GetActorTransform))
  (bind _returnvalue_3 (Transformation|GetActorTransform))
  (bind _colliderbox_rightdown (Variables|Default|GetColliderBox%20RightDown))
  (bind _colliderbox_down (Variables|Default|GetColliderBox%20Down))
  (bind _grid_size (Variables|Default|GetGrid%20Size))
  (bind _grid_size_2 (Variables|Default|GetGrid%20Size))
  (bind _colliderbox_left (Variables|Default|GetColliderBox%20Left))
  (bind _colliderbox_leftdown (Variables|Default|GetColliderBox%20LeftDown))
  (bind _colliderbox_right (Variables|Default|GetColliderBox%20Right))
  (bind _overlappingactors (Collision|GetOverlappingActors _colliderbox_right 0 :!class /Script/Engine.PrimitiveComponent))
  (bind _overlappingactors_2 (Collision|GetOverlappingActors _colliderbox_left 0 :!class /Script/Engine.PrimitiveComponent))
  (bind _overlappingactors_3 (Collision|GetOverlappingActors _colliderbox_leftdown 0 :!class /Script/Engine.PrimitiveComponent))
  (bind _overlappingactors_4 (Collision|GetOverlappingActors _colliderbox_rightdown 0 :!class /Script/Engine.PrimitiveComponent))
  (bind _overlappingactors_5 (Collision|GetOverlappingActors _colliderbox_down 0 :!class /Script/Engine.PrimitiveComponent))
  (bind _returnvalue_4 (* _grid_size -1.0))
  (bind _returnvalue_5 (* _grid_size_2 -1.0))
  (bind _returnvalue_6 (Utilities|Array|Length _overlappingactors))
  (bind _returnvalue_7 (Utilities|Array|Length _overlappingactors_2))
  (bind _returnvalue_8 (Utilities|Array|Length _overlappingactors_3))
  (bind _returnvalue_9 (Utilities|Array|Length _overlappingactors_4))
  (bind _returnvalue_10 (== _returnvalue_9 0))
  (bind _returnvalue_11 (== _returnvalue_6 0))
  (bind _returnvalue_12 (== _returnvalue_7 0))
  (bind _returnvalue_13 (== _returnvalue_8 0))
  (bind _returnvalue_14 (and _returnvalue_11 _returnvalue_10))
  (bind _returnvalue_15 (and _returnvalue_12 _returnvalue_13))
  ;[1 1 1] Prerequisites
  (if (not (Variables|Default|GetMoving)) :!label _label
    (if (== (Utilities|Array|Length _overlappingactors_5) 0)
      ;[1 1 1] Fall down
      (Variables|Default|SetMoving true)
      (bind _progress (Timeline|Drop%20Down%20Timeline Play)
        (:Update
          (Transformation|SetRelativeLocation (Variables|Default|GetSphere) (Math|Vector|MakeVector (* _progress _returnvalue_4) 0.0 0.0) false false))
        (:Finished
          (Utilities|FlowControl|Sequence
            (:then_0
              (Timeline|Drop%20Down%20Timeline SetNewTime))
            (:then_1
              (Transformation|SetActorLocation (Math|Vector|MakeVector (+ _returnvalue_4 (.x (.location _returnvalue))) (.y (.location _returnvalue)) (.z (.location _returnvalue))) false false)
              (Variables|Default|SetMoving false)
              ;[1 1 1] Check if boulder killed player
              (bind _array_element (Utilities|Array|ForEachLoopwithBreak (Collision|GetOverlappingActors (Variables|Default|GetColliderBox%20Down) "/Script/Engine.Pawn" :!class /Script/Engine.PrimitiveComponent) :!label _label_2)
                (:LoopBody
                  (bind _asi_killable (Utilities|Casting|CastToI_Killable _array_element))
                  (Default|Sepuku _asi_killable))
                (:Completed
                  (goto _label)))))))
      (else
        (bind _array_element_2 (Utilities|Array|ForEachLoopwithBreak _overlappingactors_5 :!label _label_3)
          (:LoopBody
            (if (Utilities|DoesObjectImplementInterface _array_element_2 "/Game/BoulderDash/Interfaces/I_CanFallOff.I_CanFallOff_C")
              (Utilities|FlowControl|Sequence
                (:then_0
                  (goto _label_3 Break))
                (:then_1
                  ;[1 1 1] Check fall to side
                  (if (Math|Random|RandomBool)
                    (if _returnvalue_14
                      (Variables|Default|SetLeftOrRight false :!label _label_4)
                      ;[1 1 1] Move sideways
                      (Variables|Default|SetMoving true :!label _label_5)
                      (bind _progress_2 (Timeline|Move%20Right%20Timeline Play)
                        (:Update
                          (Transformation|SetRelativeLocation (Variables|Default|GetSphere) (Math|Vector|MakeVector 0.0 (* _progress_2 (* (Variables|Default|GetGrid%20Size) (Math|Float|SelectFloat -1.0 1.0 (Variables|Default|GetLeftOrRight)))) 0.0) false false))
                        (:Finished
                          (Utilities|FlowControl|Sequence
                            (:then_0
                              (Timeline|Move%20Right%20Timeline SetNewTime))
                            (:then_1
                              (Transformation|SetActorLocation (Math|Vector|MakeVector (.x (.location _returnvalue_3)) (+ (* (Variables|Default|GetGrid%20Size) (Math|Float|SelectFloat -1.0 1.0 (Variables|Default|GetLeftOrRight))) (.y (.location _returnvalue_3))) (.z (.location _returnvalue_3))) false false)
                              ;[1 1 1] Move down
                              (bind _progress_3 (Timeline|Move%20Down%20Timeline Play)
                                (:Update
                                  (Transformation|SetRelativeLocation (Variables|Default|GetSphere) (Math|Vector|MakeVector (* _progress_3 _returnvalue_5) 0.0 0.0) false false))
                                (:Finished
                                  (Utilities|FlowControl|Sequence
                                    (:then_0
                                      (Timeline|Move%20Down%20Timeline SetNewTime))
                                    (:then_1
                                      (Transformation|SetActorLocation (Math|Vector|MakeVector (+ _returnvalue_5 (.x (.location _returnvalue_2))) (.y (.location _returnvalue_2)) (.z (.location _returnvalue_2))) false false)
                                      (Variables|Default|SetMoving false)
                                      (goto _label_2)))))))))
                      (elif _returnvalue_15
                        (Variables|Default|SetLeftOrRight true :!label _label_6)
                        (goto _label_5)))
                    (elif _returnvalue_15
                      (goto _label_6)
                      (elif _returnvalue_14
                        (goto _label_4)))))))))))))

(event EventBeginPlay
  (for _array_element (Utilities|Array|MakeArray (Variables|Default|GetDrop%20Down%20Timeline) (Variables|Default|GetMove%20Down%20Timeline) (Variables|Default|GetMove%20Right%20Timeline))
    (Components|Timeline|SetPlayRate _array_element (Variables|Default|GetAnimation%20Rate))))

(event EventOnPush
  (params (Player%20Collider%20Position :type Vector :default "0, 0, 0") (Push%20Component :type Push%20Component%20Object%20Reference) (Pawn :type Pawn%20Object%20Reference))
  (bind _returnvalue (Transformation|GetActorTransform))
  (bind _colliderbox_right (Variables|Default|GetColliderBox%20Right))
  (bind _colliderbox_left (Variables|Default|GetColliderBox%20Left))
  (bind _array (Utilities|Array|MakeArray _colliderbox_right _colliderbox_left))
  ;[1 1 1] Pushing boulders
  (for (_array_element _array_index) _array
    (if (== (Utilities|Array|Length (Collision|GetOverlappingActors _array_element 0 :!class /Script/Engine.PrimitiveComponent)) 1)
      (for _array_element_2 (Collision|GetOverlappingActors _array_element 0 :!class /Script/Engine.PrimitiveComponent)
        (if (== Pawn _array_element_2)
          (Rendering|Debug|DrawDebugSphere (.location (Math|Transform|ComposeTransforms (Utilities|Array|Get(acopy) (Variables|Default|GetPush%20Transforms) _array_index) (Transformation|GetActorTransform))) 2e+01 12 "(R=1.000000,G=0.000000,B=0.000000,A=1.000000)" 2.0 1.0)
          (if (== (Utilities|Array|Length (Collision|GetOverlappingActors (Utilities|Array|Get(acopy) _array (Math|Integer|%(Integer) (+ _array_index 1) 2)) 0 :!class /Script/Engine.PrimitiveComponent)) 0)
            (Variables|Default|SetLeftOrRight (== _array_index 0))
            ;;[1 1 1] Move sideways
            (Variables|Default|SetMoving true)
            (bind _progress (Timeline|Timeline Play)
              (:Update
                (Transformation|SetRelativeLocation (Variables|Default|GetSphere) (Math|Vector|MakeVector 0.0 (* _progress (* (Variables|Default|GetGrid%20Size) (Math|Float|SelectFloat -1.0 1.0 (Variables|Default|GetLeftOrRight)))) 0.0) false false))
              (:Finished
                (Utilities|FlowControl|Sequence
                  (:then_0
                    (Timeline|Timeline SetNewTime))
                  (:then_1
                    (Transformation|SetActorLocation (Math|Vector|MakeVector (.x (.location _returnvalue)) (+ (* (Variables|Default|GetGrid%20Size) (Math|Float|SelectFloat -1.0 1.0 (Variables|Default|GetLeftOrRight))) (.y (.location _returnvalue))) (.z (.location _returnvalue))) false false)
                    (Variables|Default|SetMoving false)
                    (CallFunction|TryFallDown)))))
            (else
              (Development|PrintString "No space on the other side to push")))
          (else
            (Development|PrintString "He not chosen one"))))
      (else
        (Development|PrintString "Wrong overlapping actors amount")))))

(fn ConstructionScript
  (for _array_element (Variables|Default|GetPush%20Transforms)
    (AddComponent|AddArrowComponent false (Math|Transform|MakeTransform (* (.Location (Math|Transform|BreakTransform _array_element)) (Math|Vector|MakeVector 1.5 1.5 1.5)) (.Rotation (Math|Transform|BreakTransform _array_element)) (.Scale (Math|Transform|BreakTransform _array_element))))))

(fn FindClosestPushTransform
  (params (Character%20Location :type Vector) (Push%20Component :type Push%20Component%20Object%20Reference))
  (bind _push_range (Variables|/Game/BoulderDash/Blueprints/PushComponent.PushComponent_C|GetPush%20Range Push%20Component))
  (bind _returnvalue (Math|Float|Square _push_range))
  (for (_array_element _array_index) (Variables|Default|GetPush%20Transforms)
    (Development|PrintString (Utilities|String|JoinStringArray (Utilities|Array|MakeArray (Utilities|String|ToString(Float) (Class|KismetMathLibrary|DistanceSquared2D (Math|Conversions|ToVector2D(Vector) (Math|Transform|TransformLocation (Transformation|GetActorTransform) (.location _array_element))) (Math|Conversions|ToVector2D(Vector) Character%20Location))) "<=" (Utilities|String|ToString(Float) _returnvalue)) " "))
    (if (<= (Class|KismetMathLibrary|DistanceSquared2D (Math|Conversions|ToVector2D(Vector) (Math|Transform|TransformLocation (Transformation|GetActorTransform) (.location _array_element))) (Math|Conversions|ToVector2D(Vector) Character%20Location)) _returnvalue)
      (return _array_index)))
  (return -1))

(fn DoesOverlapAnything
  (params (Collider%20Box :type Primitive%20Component%20Object%20Reference))
  (return (not (== (Utilities|Array|Length (Collision|GetOverlappingActors Collider%20Box 0 :!class /Script/Engine.PrimitiveComponent)) 0))))