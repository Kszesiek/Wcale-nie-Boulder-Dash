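; Quicksand hazard for BoulderDash that captures pawns entering its collision volume and makes them fall through it.
; On overlap it zeroes the third-person character's gravity, while a timeline pulls any pawn horizontally toward the quicksand's center.
; When the timeline finishes, it sets a vertical fall velocity and flags the pawn through I_CanFallFromQuicksand.
; Leaving the volume restores a hardcoded gravity scale for the character and clears the falling flag.
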(event OnComponentBeginOverlap(CollisionOverlap)
  (params (OverlappedComponent :type Primitive%20Component%20Object%20Reference) (OtherActor :type Actor%20Object%20Reference) (OtherComp :type Primitive%20Component%20Object%20Reference) (OtherBodyIndex :type Integer) (bFromSweep :type Boolean) (SweepResult :type Hit%20Result%20Structure%20%28by%20ref%29))
  (Utilities|FlowControl|Sequence
    (:then_0
      (bind _asbp_third_person_character (Utilities|Casting|CastToBP_ThirdPersonCharacter OtherActor))
      (Variables|/Script/Engine.CharacterMovementComponent|SetGravityScale (Variables|/Script/Engine.Character|GetCharacterMovement _asbp_third_person_character) 0.0))
    (:then_1
      (bind _aspawn (Utilities|Casting|CastToPawn OtherActor))
      ;[1 1 1] Move actor to the middle of quicksand
      (bind _progress (Timeline|MoveToCenter%20Timeline Play)
        (:Update
          (Transformation|SetActorLocation _aspawn (Math|Vector|MakeVector (.x (+ (* _progress (- (Transformation|GetActorLocation) (Transformation|GetActorLocation _aspawn))) (Transformation|GetActorLocation _aspawn))) (.y (+ (* _progress (- (Transformation|GetActorLocation) (Transformation|GetActorLocation _aspawn))) (Transformation|GetActorLocation _aspawn))) (.Z (Math|Vector|BreakVector (Transformation|GetActorLocation _aspawn)))) false false))
        (:Finished
          ;[1 1 1] The "falling" part
          (bind _asi_can_fall_from_quicksand (Utilities|Casting|CastToI_CanFallFromQuicksand _aspawn)
            (:then
              (Default|SetIsFallingfromQuicksand _asi_can_fall_from_quicksand true))
            (:CastFailed
              _))
          (Variables|/Script/Engine.MovementComponent|SetVelocity (Pawn|GetMovementComponent _aspawn) (Math|Vector|MakeVector 0.0 0.0 (Variables|Default|GetFall%20velocity))))))))

(event OnComponentEndOverlap(CollisionOverlap)
  (params (OverlappedComponent :type Primitive%20Component%20Object%20Reference) (OtherActor :type Actor%20Object%20Reference) (OtherComp :type Primitive%20Component%20Object%20Reference) (OtherBodyIndex :type Integer))
  (Utilities|FlowControl|Sequence
    (:then_0
      (bind _asbp_third_person_character (Utilities|Casting|CastToBP_ThirdPersonCharacter OtherActor))
      (Variables|/Script/Engine.CharacterMovementComponent|SetGravityScale (Variables|/Script/Engine.Character|GetCharacterMovement _asbp_third_person_character) 1.75))
    (:then_1
      (bind _asi_can_fall_from_quicksand (Utilities|Casting|CastToI_CanFallFromQuicksand OtherActor))
      (Default|SetIsFallingfromQuicksand _asi_can_fall_from_quicksand false))))

(fn ConstructionScript)