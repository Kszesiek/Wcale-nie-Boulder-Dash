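; Key is a collectible item actor that idles with a bob and spin and plays a choir sound when destroyed.
; A looping timeline drives the key component's sine-based height, scaled by JumpHeight, and a full yaw rotation per cycle.
; GetItemName both destroys the actor and returns its Name, so querying the name acts as the pickup.
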(event EventBeginPlay
  (bind _animation (Timeline|Idle%20Animation%20Timeline Play)
    (:Update
      (Transformation|SetRelativeLocationAndRotation (Variables|Default|GetKey) (Math|Vector|MakeVector 0.0 0.0 (* (Math|Trig|Sin(Radians) (* (Math|Float|%(Float) _animation 0.5) (Math|Trig|GetPI) 4.0)) (Variables|Default|GetJump%20Height))) (Math|Rotator|MakeRotator 0.0 0.0 (* _animation 3.6e+02)) false false))
    (:Finished
      (Timeline|Idle%20Animation%20Timeline PlayFromStart))))

(event EventDestroyed
  (Audio|PlaySound2D "/Game/BoulderDash/Sounds/angel-choirrr.angel-choirrr" 1.0 1.0 0.0 0 0))

(fn ConstructionScript)

(fn GetItemName
  (Actor|DestroyActor)
  (return (Variables|Default|GetName)))