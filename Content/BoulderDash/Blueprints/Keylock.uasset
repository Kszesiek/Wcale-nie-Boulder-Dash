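; Keylock actor for BoulderDash that a collector opens by spending the collectable it requires.
; On box overlap, it looks for its Name in the collectables of an I_Collector actor, uses that collectable and destroys itself.
; When destroyed, it sends an unlock message to its parent actor if that implements I_Lockable, so it works as a child actor of a lockable object.
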(event OnComponentBeginOverlap(BoxCollision)
  (params (OverlappedComponent :type Primitive%20Component%20Object%20Reference) (OtherActor :type Actor%20Object%20Reference) (OtherComp :type Primitive%20Component%20Object%20Reference) (OtherBodyIndex :type Integer) (bFromSweep :type Boolean) (SweepResult :type Hit%20Result%20Structure%20%28by%20ref%29))
  (if (Utilities|DoesObjectImplementInterface OtherActor "/Game/BoulderDash/Interfaces/I_Collector.I_Collector_C")
    (bind _collectables_list (Class|ICollector|GetCollectables(Message) OtherActor))
    (if (>= (Utilities|Array|FindItem _collectables_list (Variables|Default|GetName)) 0)
      (Class|ICollector|UseCollectable(Message) OtherActor (Variables|Default|GetName))
      (Actor|DestroyActor))))

(event EventDestroyed
  (bind _returnvalue (Actor|GetParentActor))
  (if (Utilities|DoesObjectImplementInterface _returnvalue "/Game/BoulderDash/Interfaces/I_Lockable.I_Lockable_C")
    (Class|ILockable|UnlockSelf(Message) _returnvalue)))

(fn ConstructionScript)